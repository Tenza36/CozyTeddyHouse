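; BP_Pierna is an unfinished interactable Blueprint in the Peluches folder that enables player 0 input on BeginPlay.
; IA_Interact runs a Visibility line trace from the player controller's location along a forward vector scaled by Distance, without using the result.
; The trace and the Hit event both lead into a SelfMoved branch that does nothing yet.
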(event Input|EnhancedActionEvents|EnhancedInputActionIA_Interact
  (params (ActionValue :type Boolean) (ElapsedSeconds :type Float%20%28double-precision%29) (TriggeredSeconds :type Float%20%28double-precision%29) (InputAction :type Input%20Action%20Object%20Reference :default "/Game/FirstPerson/Input/Actions/IA_Interact.IA_Interact"))
  (bind _returnvalue (Game|GetPlayerController 0))
  (bind _returnvalue_2 (Transformation|GetActorLocation _returnvalue))
  (Collision|LineTraceByChannel _returnvalue_2 (+ _returnvalue_2 (* (Variables|Default|Getdistance) (Class|KismetMathLibrary|VectorForward))) "TraceTypeQuery1" false 0 "None")
  (if (stale Collision|EventHit bSelfMoved)
    _))

(event EventBeginPlay
  (Input|EnableInput (Game|GetPlayerController 0)))

(event Collision|EventActorBeginOverlap
  (params (OtherActor :type Actor%20Object%20Reference)))

(event EventTick
  (params (DeltaSeconds :type Float%20%28single-precision%29)))

(event Collision|EventHit
  (params (MyComp :type Primitive%20Component%20Object%20Reference) (Other :type Actor%20Object%20Reference) (OtherComp :type Primitive%20Component%20Object%20Reference) (bSelfMoved :type Boolean) (HitLocation :type Vector :default "0, 0, 0") (HitNormal :type Vector :default "0, 0, 0") (NormalImpulse :type Vector :default "0, 0, 0") (Hit :type Hit%20Result%20Structure%20%28by%20ref%29))
  (if bSelfMoved
    _))

(fn ConstructionScript)