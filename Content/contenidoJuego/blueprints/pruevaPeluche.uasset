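; Test plush toy (peluche) actor assembled from six static mesh parts: legs, torso, arms, eyes, head and ears.
; BeginPlay stores those components in Objetivo.
; GenerarstructDesdeActor packs the body-part mesh and material arrays into a composite plush struct by fixed indices.
; ConfigurarDesdeStruct applies such a struct to the components, with field names that do not match their target parts (e.g. Brazos drives Torso).
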(event EventBeginPlay
  (Variables|Default|Setobjetivo (Utilities|Array|MakeArray (Variables|Default|Getpiernass) (Variables|Default|Gettorso) (Variables|Default|Getbrazoss) (Variables|Default|Getojos) (Variables|Default|Getcabeza) (Variables|Default|Getorejas))))

(event EventTick
  (params (DeltaSeconds :type Float%20%28single-precision%29)))

(fn ConstructionScript)

(fn GenerarstructDesdeActor
  (bind _materialespartescuerpo (Variables|Default|Getmaterialespartescuerpo))
  (bind _meshpartescuerpo (Variables|Default|Getmeshpartescuerpo))
  (return (Utilities|Struct|Makepeluchecompuestostruct 0 (Utilities|Struct|MakePeluchesStruct "" (Utilities|Array|Get(acopy) _meshpartescuerpo 4) (Utilities|Array|Get(acopy) _materialespartescuerpo 4)) (Utilities|Struct|MakePeluchesStruct "" (Utilities|Array|Get(acopy) _meshpartescuerpo 5) (Utilities|Array|Get(acopy) _materialespartescuerpo 5)) (Utilities|Struct|MakePeluchesStruct "" (Utilities|Array|Get(acopy) _meshpartescuerpo 1) (Utilities|Array|Get(acopy) _materialespartescuerpo 1)) (Utilities|Struct|MakePeluchesStruct "" (Utilities|Array|Get(acopy) _meshpartescuerpo) (Utilities|Array|Get(acopy) _materialespartescuerpo)) (Utilities|Struct|MakePeluchesStruct "" (Utilities|Array|Get(acopy) _meshpartescuerpo 2) (Utilities|Array|Get(acopy) _materialespartescuerpo 2)) (Utilities|Struct|MakePeluchesStruct "" (Utilities|Array|Get(acopy) _meshpartescuerpo 3) (Utilities|Array|Get(acopy) _materialespartescuerpo 3)))))

(fn ConfigurarDesdeStruct
  (params (fatos%20del%20peluche :type Peluchecompuestostruct%20Structure))
  (bind (_numbre _cabeza _torso _piernas _brazos _nariz _boca) (Utilities|Struct|Breakpeluchecompuestostruct fatos%20del%20peluche))
  (bind _orejas (Variables|Default|Getorejas))
  (bind _torso_2 (Variables|Default|Gettorso))
  (bind _brazoss (Variables|Default|Getbrazoss))
  (bind _ojos (Variables|Default|Getojos))
  (bind _cabeza_2 (Variables|Default|Getcabeza))
  (bind _piernass (Variables|Default|Getpiernass))
  (bind (_nombre _mesh _material) (Utilities|Struct|BreakPeluchesStruct _torso))
  (bind (_nombre_2 _mesh_2 _material_2) (Utilities|Struct|BreakPeluchesStruct _brazos))
  (bind (_nombre_3 _mesh_3 _material_3) (Utilities|Struct|BreakPeluchesStruct _piernas))
  (bind (_nombre_4 _mesh_4 _material_4) (Utilities|Struct|BreakPeluchesStruct _nariz))
  (bind (_nombre_5 _mesh_5 _material_5) (Utilities|Struct|BreakPeluchesStruct _boca))
  (bind (_nombre_6 _mesh_6 _material_6) (Utilities|Struct|BreakPeluchesStruct _cabeza))
  (Components|StaticMesh|SetStaticMesh _torso_2 _mesh_2)
  (Rendering|Material|SetMaterial _torso_2 0 _material_2)
  (Components|StaticMesh|SetStaticMesh _cabeza_2 _mesh_3)
  (Rendering|Material|SetMaterial _cabeza_2 0 _material_3)
  (Components|StaticMesh|SetStaticMesh _orejas _mesh_4)
  (Rendering|Material|SetMaterial _orejas 0 _material_4)
  (Components|StaticMesh|SetStaticMesh _brazoss _mesh_5)
  (Rendering|Material|SetMaterial _brazoss 0 _material_5)
  (Components|StaticMesh|SetStaticMesh _piernass _mesh_6)
  (Rendering|Material|SetMaterial _piernass 0 _material_6)
  (Components|StaticMesh|SetStaticMesh _ojos _mesh)
  (Rendering|Material|SetMaterial _ojos 0 _material)
  (return))