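; Display table where the player places a plush from their inventory to sell at a set price.
; Overlap enables input and a prompt; R spawns a PruevaPeluche from the selected inventory struct, removes that entry and updates the character's counters.
; It then opens a Priceset widget with mouse cursor and look locked.
; IaCogePeluche destroys a plush and pays Precio into the player's Dinero; logic returning plushes to inventory is unconnected.
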(event Collision|EventActorEndOverlap
  (params (OtherActor :type Actor%20Object%20Reference))
  ;[1 1 1] abilitador de inputs de mesa de colocacion
  (Input|DisableInput 0)
  (Variables|Default|Setpuedecolocar false)
  (bind _asbp_first_person_character (Utilities|Casting|CastToBP_FirstPersonCharacter (Game|Player|GetPlayerPawn 0)))
  (Variables|/Game/FirstPerson/Blueprints/BP_FirstPersonCharacter.BP_FirstPersonCharacter_C|SetTexto _asbp_first_person_character " "))

(event Collision|EventActorBeginOverlap
  (params (OtherActor :type Actor%20Object%20Reference))
  ;[1 1 1] abilitador de inputs de mesa de colocacion
  (bind _newparam (CallFunction|NewFunction))
  (if (> (Variables|/Game/FirstPerson/Blueprints/BP_FirstPersonCharacter.BP_FirstPersonCharacter_C|Getcontadorinventario _newparam) 0)
    (Input|EnableInput (Game|GetPlayerController 0))
    (Variables|Default|Setpuedecolocar true)
    (bind _asbp_first_person_character (Utilities|Casting|CastToBP_FirstPersonCharacter (Game|Player|GetPlayerPawn 0)))
    (Variables|/Game/FirstPerson/Blueprints/BP_FirstPersonCharacter.BP_FirstPersonCharacter_C|SetTexto _asbp_first_person_character "press R to place ")))

(event Input|KeyboardEvents|R
  (params (Key :type Key%20Structure :default "None"))
  (bind _returnvalue (Game|GetPlayerController 0))
  (bind _cube (Variables|Default|GetCube))
  (:Pressed
    (bind _newparam (CallFunction|NewFunction))
    (if (> (Variables|/Game/FirstPerson/Blueprints/BP_FirstPersonCharacter.BP_FirstPersonCharacter_C|Getcontadorinventario _newparam) 0)
      (Utilities|FlowControl|FlipFlop
        (:A
          (Variables|Default|Setpeluches%20colocables (- (Variables|Default|Getpeluches%20colocables) 1))
          (bind _asbp_first_person_character (Utilities|Casting|CastToBP_FirstPersonCharacter (Game|Player|GetPlayerPawn 0)))
          (if (not (Variables|Default|Getcolocado))
            (if (Variables|Default|Getpuedecolocar)
              (bind _returnvalue_2 (Game|SpawnActorfromClass "/Game/contenidoJuego/blueprints/pruevaPeluche.pruevaPeluche_C" (Math|Transform|MakeTransform (Transformation|GetWorldLocation _cube) (Transformation|GetWorldRotation _cube) "0.300000,0.300000,0.300000") "Undefined" "MultiplyWithRoot" 0 0 0 0 0))
              (Default|ConfigurarDesdeStruct _returnvalue_2 (Utilities|Array|Get(acopy) (Variables|/Game/FirstPerson/Blueprints/BP_FirstPersonCharacter.BP_FirstPersonCharacter_C|Getinventariopeluche _asbp_first_person_character) (Variables|/Game/FirstPerson/Blueprints/BP_FirstPersonCharacter.BP_FirstPersonCharacter_C|Getnumerodeinventarioseleccionado _asbp_first_person_character)))
              (Utilities|Array|RemoveIndex (Variables|/Game/FirstPerson/Blueprints/BP_FirstPersonCharacter.BP_FirstPersonCharacter_C|Getinventariopeluche _asbp_first_person_character) (Variables|/Game/FirstPerson/Blueprints/BP_FirstPersonCharacter.BP_FirstPersonCharacter_C|Getnumerodeinventarioseleccionado _asbp_first_person_character))
              (bind _asbp_first_person_character_2 (Utilities|Casting|CastToBP_FirstPersonCharacter (Game|Player|GetPlayerPawn 0)))
              (bind _output_get (Variables|/Game/FirstPerson/Blueprints/BP_FirstPersonCharacter.BP_FirstPersonCharacter_C|Setnumerodelpelucheenedicion _asbp_first_person_character_2 (+ (Variables|/Game/FirstPerson/Blueprints/BP_FirstPersonCharacter.BP_FirstPersonCharacter_C|Getnumerodelpelucheenedicion _asbp_first_person_character_2) 1)))
              (Variables|/Game/FirstPerson/Blueprints/BP_FirstPersonCharacter.BP_FirstPersonCharacter_C|Setcontadorinventario _asbp_first_person_character_2 (+ -1 (Variables|/Game/FirstPerson/Blueprints/BP_FirstPersonCharacter.BP_FirstPersonCharacter_C|Getcontadorinventario _asbp_first_person_character_2)))
              (Variables|Default|Setcolocado true)
              (Variables|Default|Setpeluche%20en%20mesa _output_get)
              (Variables|Default|Setpuedecolocar false)
              (Variables|Default|Setcolocado true)
              (bind _returnvalue_3 (UserInterface|CreateWidget "/Game/contenidoJuego/blueprints/priceset.priceset_C"))
              (Variables|/Game/contenidoJuego/blueprints/priceset.priceset_C|Setmesa _returnvalue_3 self)
              (UserInterface|Viewport|AddtoViewport _returnvalue_3 0)
              (Variables|Default|Setprecio (Variables|/Game/contenidoJuego/blueprints/priceset.priceset_C|Getprecio%20ingresado _returnvalue_3))
              (Variables|/Script/Engine.PlayerController|SetbShowMouseCursor _returnvalue true)
              (Input|SetIgnoreLookInput _returnvalue true)
              (Variables|Default|Setreferencia%20a%20priceset _returnvalue_3)
              (CallFunction|WidgetVisibility true)
              (bind _asbp_first_person_character_3 (Utilities|Casting|CastToBP_FirstPersonCharacter (Game|Player|GetPlayerPawn 0)))
              (Variables|/Game/FirstPerson/Blueprints/BP_FirstPersonCharacter.BP_FirstPersonCharacter_C|SetTexto _asbp_first_person_character_3 " "))))))))

(fn ConstructionScript)

(fn NewFunction
  (bind _asbp_first_person_character (Utilities|Casting|CastToBP_FirstPersonCharacter (Game|GetPlayerCharacter 0)))
  (return _asbp_first_person_character))

(fn IaCogePeluche
  (bind _newparam (CallFunction|NewFunction))
  (bind _outactors (Actor|GetAllActorsOfClass "/Game/contenidoJuego/blueprints/pruevaPeluche.pruevaPeluche_C"))
  (bind _returnvalue (Actor|GetActorOfClass (Utilities|GetClass (Utilities|Array|Get(acopy) _outactors (Variables|Default|Getpeluche%20en%20mesa)))))
  (Actor|DestroyActor _returnvalue)
  (Variables|/Game/FirstPerson/Blueprints/BP_FirstPersonCharacter.BP_FirstPersonCharacter_C|SetDinero _newparam (+ (Variables|/Game/FirstPerson/Blueprints/BP_FirstPersonCharacter.BP_FirstPersonCharacter_C|GetDinero _newparam) (Variables|Default|Getprecio))))

(fn WidgetVisibility
  (params (NewParam :type Boolean))
  (bind _referencia_a_priceset (Variables|Default|Getreferencia%20a%20priceset))
  (if NewParam
    (Widget|SetVisibility _referencia_a_priceset "Visible")
    (else
      (Widget|SetVisibility _referencia_a_priceset "Hidden"))))