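; Spawn manager actor that spawns a set of actors around itself when the IA_Spawn input fires.
; BeginPlay enables input from player controller 0, and the input event calls SpawnSet.
; SpawnSet spawns each class in the BPCabeza array at one tenth scale, offset one unit from the manager in a random direction, with a random rotation without roll.
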(event Input|EnhancedActionEvents|EnhancedInputActionIA_Spawn
  (params (ActionValue :type Boolean) (ElapsedSeconds :type Float%20%28double-precision%29) (TriggeredSeconds :type Float%20%28double-precision%29) (InputAction :type Input%20Action%20Object%20Reference :default "/Game/FirstPerson/Input/Actions/IA_Spawn.IA_Spawn"))
  (CallFunction|SpawnSet))

(event EventBeginPlay
  (Input|EnableInput (Game|GetPlayerController 0)))

(event Collision|EventActorBeginOverlap
  (params (OtherActor :type Actor%20Object%20Reference)))

(event EventTick
  (params (DeltaSeconds :type Float%20%28single-precision%29)))

(fn ConstructionScript)

(fn SpawnSet
  (for _array_element (Variables|Default|GetBP_Cabeza)
    (Game|SpawnActorfromClass _array_element (Math|Transform|MakeTransform (+ (Math|Random|RandomUnitVector) (Transformation|GetActorLocation)) (Math|Random|RandomRotator false) "0.100000,0.100000,0.100000") "Undefined" "MultiplyWithRoot" 0 0)))